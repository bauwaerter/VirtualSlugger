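; Baseball bat actor that takes its rotation from a Femtoduino device.
; Tick accumulates delta time and, each time it reaches the Max interval, sets the actor rotation from GetQRotation and prints the value.
; It then calls WriteFemtoduino and resets the timer; the first interval skips the rotation and only performs the write.
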(event `self.ReceiveTick`
  (params (DeltaSeconds :type "Float (single-precision)"))
  (bind _current (`self.Current`))
  (`/Engine/EditorBlueprintResources/StandardMacros.CompareFloat` _current (`self.Max`)
    (:`>`
      (if (`self.IsFirst`) :!label _label
        (set `self.IsFirst` false)
        (else
          (bind _returnvalue (`Libraries.GetQRotation`))
          (`KismetSystemLibrary.PrintString` (`KismetStringLibrary.Conv_RotatorToString` _returnvalue) true true (struct :`R` 1.0 :`G` 0.070607 :`A` 1.0))
          (`self.SetActorRotation` _returnvalue)))
      (`Libraries.WriteFemtoduino`)
      (set `self.Current` 0.0))
    (:`==`
      (goto _label))
    (:`<`
      (set `self.Current` (+ DeltaSeconds _current)))))

(fn `UserConstructionScript`)