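; NewGameMode is a game mode Blueprint that spawns a baseball bat for the batter through the SetBatter event.
; The event converts BatSide to a side value and spawns Baseball_bat at the matching left or right location, using Batsize as scale.
; Batsize is always reset to unit scale, because the switch on BatSize that would offer a doubled scale is disconnected and never runs.
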(event `SetBatter`
  (params (BatSize :type Byte) (BatSide :type Byte))
  (bind (_leftlocation_location _leftlocation_rotation) (`KismetMathLibrary.BreakTransform` (`self.LeftLocation`)))
  (bind (_rightlocation_location _rightlocation_rotation) (`KismetMathLibrary.BreakTransform` (`self.RightLocation`)))
  ;[1 1 1] Setting Bat Size
  (set `self.Batsize` (1.0 1.0 1.0))
  ;[1 1 1] Setting Bat Side
  (switch `/Game/Menu/NewWidgets/BatSide` (cast `/Game/Menu/NewWidgets/BatSide` BatSide)
    (:`NewEnumerator0`
      (`|SpawnActorFromClass` "/Game/Blueprints/baseball_bat.baseball_bat_C" (`KismetMathLibrary.MakeTransform` _leftlocation_location _leftlocation_rotation (`self.Batsize`)) false 1.0))
    (:`NewEnumerator1`
      (`|SpawnActorFromClass` "/Game/Blueprints/baseball_bat.baseball_bat_C" (`KismetMathLibrary.MakeTransform` _rightlocation_location _rightlocation_rotation (`self.Batsize`)) false 1.0))))

(fn `UserConstructionScript`)